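; BP_PMPC is a player controller that handles touch input setup and the respawn UI hook.
; MobileInputSetup activates the thumb gamepad touch interface, then shows the mouse cursor when the platform user name matches "Windows".
; OnRespawn opens the death screen through the common UI manager and prints a debug string.
; BeginPlay only runs a brief delay, and an ad banner call is left disconnected.
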(event EventBeginPlay
  (Utilities|FlowControl|Delay 0.001))

(event EventMobileInputSetup
  (Class|PlayerController|ActivateTouchInterface "/Game/CommonUI/TI_ThumbGameController.TI_ThumbGameController")
  (switch string (Utilities|Platform|GetPlatformUserName)
    (:Windows
      (if true
        (Variables|Default|SetbShowMouseCursor true)
        (Development|PrintString "Hello")))))

(event EventOnRespawn
  (Class|PMCommonUIManager|ActivateDeathScreen (Variables|Default|GetBP_PM_CommonUIManager))
  (Development|PrintString "Hello"))

(fn ConstructionScript)