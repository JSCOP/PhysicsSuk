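; BP_PhysicsAxisLockActor is a physics-driven actor that spins two gear components in opposite roll directions as it moves.
; Each tick, the rounded Y component of the normalized movement since the last stored location sets the spin direction.
; The magnitude of RootPhysicsMesh's angular velocity in radians sets the per-tick rotation step, applied directly as degrees without delta-time scaling.
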(event EventBeginPlay
  (Variables|Default|SetPastLocation (Transformation|GetActorLocation)))

(event EventTick
  (params (DeltaSeconds :type Float%20%28single-precision%29))
  (Utilities|FlowControl|Sequence
    (:then_0
      (Transformation|AddLocalRotation (Variables|Default|GetGear) (Math|Rotator|MakeRotator (* (Math|Float|Round (.y (Math|Vector|Normalize (- (Transformation|GetActorLocation) (Variables|Default|GetPastLocation))))) (Math|Vector|VectorLength (Class|PrimitiveComponent|GetPhysicsAngularVelocityinRadians (Variables|Default|GetRootPhysicsMesh) "None"))) 0.0 0.0) false false))
    (:then_1
      (Transformation|AddLocalRotation (Variables|Default|GetGear1) (Math|Rotator|MakeRotator (* (* (Math|Float|Round (.y (Math|Vector|Normalize (- (Transformation|GetActorLocation) (Variables|Default|GetPastLocation))))) (Math|Vector|VectorLength (Class|PrimitiveComponent|GetPhysicsAngularVelocityinRadians (Variables|Default|GetRootPhysicsMesh) "None"))) -1.0) 0.0 0.0) false false)
      (Variables|Default|SetPastLocation (Transformation|GetActorLocation)))))

(fn ConstructionScript)